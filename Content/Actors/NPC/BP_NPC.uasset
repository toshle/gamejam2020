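; BP_NPC is an NPC actor with a swappable skeletal mesh, applied from Model on construction or through ChangeModel.
; PlayRandomGesture uses the Enemy flag to choose an animation map, then plays the animation keyed by the current mesh.
; A successful gesture also plays a quiet random sound at the mesh, so only the sound is randomized.
; TriggerTimeline animates the materials' "Amount" parameter, then destroys the actor.
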(event Custom|Trigger%20Timeline
  (bind _amount (Timeline|Timeline_0 Play)
    (:Update
      (Rendering|Material|SetScalarParameterValueonMaterials (Variables|Character|GetMesh) "Amount" _amount))
    (:Finished
      (Actor|DestroyActor))))

(fn ConstructionScript
  (Class|SkinnedMeshComponent|SetSkeletalMesh (Variables|Character|GetMesh) (Variables|Default|GetModel) true))

(fn ChangeModel
  (params (Model :type Skeletal%20Mesh%20Object%20Reference))
  (Class|SkinnedMeshComponent|SetSkeletalMesh (Variables|Character|GetMesh) Model true))

(fn PlayRandomGesture
  (bind _mesh (Variables|Character|GetMesh))
  (bind _sounds (Variables|Default|GetSounds))
  (bind _animationsmap (Variables|Default|GetAnimationsMap))
  (bind _mesh_2 (Variables|Character|GetMesh))
  (bind _enemyanimationsmap (Variables|Default|GetEnemyAnimationsMap))
  (bind _skeletalmesh (Variables|/Script/Engine.SkinnedMeshComponent|GetSkeletalMesh _mesh_2))
  (bind (_value _returnvalue) (Utilities|Map|Find _enemyanimationsmap _skeletalmesh))
  (bind (_value_2 _returnvalue_2) (Utilities|Map|Find _animationsmap _skeletalmesh))
  (if (Variables|Default|GetEnemy)
    (if _returnvalue
      (bind _asanim_sequence (Utilities|Casting|CastToAnimSequence _value)
        (:then
          (Components|Animation|PlayAnimation _mesh _asanim_sequence false)
          (Audio|PlaySoundatLocation (Utilities|Array|Get(acopy) _sounds (Math|Random|RandomInteger (Utilities|Array|Length _sounds))) (Transformation|GetWorldLocation _mesh) (Transformation|GetWorldRotation _mesh) 0.1 :!label _label))
        (:CastFailed
          (Development|PrintString "cast of anim failed" :!label _label_2)))
      (else
        (Development|PrintString "not found mesh" :!label _label_3)))
    (elif _returnvalue_2
      (bind _asanim_sequence_2 (Utilities|Casting|CastToAnimSequence _value_2)
        (:then
          (Components|Animation|PlayAnimation _mesh _asanim_sequence_2 false)
          (goto _label))
        (:CastFailed
          (goto _label_2)))
      (else
        (goto _label_3)))))