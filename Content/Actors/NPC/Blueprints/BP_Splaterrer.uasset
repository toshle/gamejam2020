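; BP_Splaterrer adds splatter effects to its owner on hit, working through the owner's capsule component.
; OnHit attaches a randomly sized, short-lived decal and a direction-aligned particle emitter, which is set to deactivate by timer.
; Particle collisions spawn smaller decals on the impacted surfaces, oriented by the hit normal.
; Each decal uses a dynamic material instance with a random Frame parameter to vary the splatter.
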(event Custom|OnHit
  (params (Direction :type Vector) (Location :type Vector) (Artist :type BP%20Artist%20Object%20Reference))
  (bind _returnvalue (Components|GetOwner))
  (bind _returnvalue_2 (Actor|GetComponentbyClass _returnvalue "/Script/Engine.CapsuleComponent"))
  (bind _returnvalue_3 (Transformation|GetWorldLocation _returnvalue_2))
  (bind _returnvalue_4 (- Location _returnvalue_3))
  (Utilities|FlowControl|Sequence
    (:then_0
      (bind _returnvalue_5 (Rendering|Material|CreateDynamicMaterialInstance "/Game/Actors/NPC/Art/Materials/M_Splatter_Decal.M_Splatter_Decal" :!class /Script/Engine.KismetMaterialLibrary))
      (Rendering|Material|SetScalarParameterValue _returnvalue_5 "Frame" (Math|Conversions|ToFloat(Integer) (Math|Random|RandomInteger 8)) :!class /Script/Engine.MaterialInstanceDynamic)
      (Class|GameplayStatics|SpawnDecalAttached _returnvalue_5 (Math|Conversions|ToVector(Float) (Math|Random|RandomFloatinRange 3e+01 4e+01)) _returnvalue_2 "None" _returnvalue_4 (Math|Conversions|RotationFromXVector "0, 0, 0") "SnapToTargetIncludingScale" 2e+01))
    (:then_1
      (bind _returnvalue_6 (Effects|SpawnEmitterAttached (Variables|Default|GetSplatterEmitters) _returnvalue_2 "None" _returnvalue_4 (Math|Conversions|RotationFromXVector Direction) "SnapToTargetIncludingScale"))
      (EventDispatchers|BindEventtoOnParticleCollide _returnvalue_6 (delegate Custom|CustomEvent_1))
      (Utilities|Time|SetTimerbyFunctionName _returnvalue_6 "Deactivate" 2.0))))

(event Custom|CustomEvent_1
  (params (EventName :type Name) (EmitterTime :type Float%20%28single-precision%29) (ParticleTime :type Integer) (Location :type Vector) (Velocity :type Vector) (Direction :type Vector) (Normal :type Vector) (BoneName :type Name) (PhysMat :type Physical%20Material%20Object%20Reference))
  ;[1 1 1] Use for later for blood trail
  (bind _returnvalue (Rendering|Material|CreateDynamicMaterialInstance "/Game/Actors/NPC/Art/Materials/M_Splatter_Decal.M_Splatter_Decal" :!class /Script/Engine.KismetMaterialLibrary))
  (Rendering|Material|SetScalarParameterValue _returnvalue "Frame" (Math|Conversions|ToFloat(Integer) (Math|Random|RandomInteger 8)) :!class /Script/Engine.MaterialInstanceDynamic)
  (Rendering|Decal|SpawnDecalatLocation _returnvalue (Math|Conversions|ToVector(Float) (Math|Random|RandomFloatinRange 1e+01 2e+01)) Location (Math|Conversions|RotationFromXVector (* Normal -1)) 2e+01))