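; BP_Painting is a painting actor that releases an enemy NPC and can take it back.
; The construction script applies materials to its background, enemy and silhouette layers.
; SpawnFromPainting sets the enemy layer's Amount parameter, then spawns BP_NPC at SpawnPoint with the chosen model and links its return component to this painting.
; ReturnToPainting plays a timeline that animates that same material parameter.
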(event Custom|Trigger%20Timeline
  (bind _amount (Timeline|Timeline_0 Play)
    (:Update
      (Rendering|Material|SetScalarParameterValueonMaterials (Variables|Default|GetEnemyPainting) "Amount" _amount))))

(fn ConstructionScript
  (Utilities|FlowControl|Sequence
    (:then_0
      (Rendering|Material|SetMaterial (Variables|Default|GetPaintingBackground) 0 (Variables|Default|GetEmptyPaintingMaterial)))
    (:then_1
      (Rendering|Material|SetMaterial (Variables|Default|GetEnemyPainting) 0 (Variables|Default|GetEnemy%20Material%20Instance)))
    (:then_2
      (Rendering|Material|SetMaterial (Variables|Default|GetEnemySilhouette) 0 (Variables|Default|GetEnemySilhouetteMaterial)))))

(fn ReturntoPainting
  (CallFunction|TriggerTimeline))

(fn SpawnfromPainting
  (bind _spawnpoint (Variables|Default|GetSpawnPoint))
  (if (Utilities|IsValid _spawnpoint)
    (Rendering|Material|SetScalarParameterValueonMaterials (Variables|Default|GetEnemyPainting) "Amount" 2.0)
    (bind _returnvalue (Game|SpawnActorfromClass "/Game/NPC/BP_NPC.BP_NPC_C" (Transformation|GetActorTransform _spawnpoint) "Undefined" 0 0))
    (Default|ChangeModel _returnvalue (Variables|Default|GetModel))
    (Variables|/Game/NPC/BP_NPC.BP_NPC_C|SetEnemy _returnvalue true)
    (Variables|/Game/Actors/Painting/Blueprints/BP_Return_To_Painting_Component.BP_Return_To_Painting_Component_C|SetPainting (Actor|GetComponentbyClass _returnvalue "/Game/Actors/Painting/Blueprints/BP_Return_To_Painting_Component.BP_Return_To_Painting_Component_C") self)))