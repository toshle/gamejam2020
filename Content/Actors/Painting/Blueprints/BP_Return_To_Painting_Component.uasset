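; Component that gives its owning actor health and, on death, returns it to its linked painting.
; OnHit forwards hit direction and location to the owner's BP_Splaterrer component, if present, then applies fixed damage to the owner's AI controller.
; The damage returned reduces Health; at zero or below, it calls ReturnToPainting on the BP_Painting and destroys the owner, provided the cast succeeds.
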(fn OnHit
  (params (HitDirection :type Vector) (HitLocation :type Vector))
  (bind _returnvalue (Components|GetOwner))
  (bind _returnvalue_2 (Actor|GetComponentbyClass _returnvalue "/Game/NPC/Blueprints/BP_Splaterrer.BP_Splaterrer_C"))
  (if (Utilities|IsValid _returnvalue_2)
    (Default|OnHit _returnvalue_2 HitDirection HitLocation))
  (bind _returnvalue_3 (Game|Damage|ApplyDamage (AI|GetAIController (Components|GetOwner)) 2e+01 0 0))
  (bind _output_get (Variables|Default|SetHealth (- (Variables|Default|GetHealth) _returnvalue_3)))
  (if (<= _output_get 0.0)
    (bind _asbp_painting (Utilities|Casting|CastToBP_Painting (Variables|Default|GetPainting)))
    (Default|ReturntoPainting _asbp_painting)
    (Actor|DestroyActor (Components|GetOwner))))