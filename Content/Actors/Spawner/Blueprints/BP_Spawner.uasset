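; Level spawner actor that populates the game at BeginPlay with painting-driven spawns and innocent NPCs.
; It first calls SpawnFromPainting on each listed BP_Painting, then scatters several BP_NPC around each innocent spawn point within a debug-drawn box.
; Each NPC gets a random yaw and skeletal mesh, is flagged non-enemy, and is skipped if no collision-free placement exists.
; An unconnected SpawnAIFromClass node using BT_NPC remains unused.
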(event EventBeginPlay
  (bind _innocentspawnradius (Variables|Default|GetInnocentSpawnRadius))
  (bind _returnvalue (Math|Vector|MakeVector _innocentspawnradius _innocentspawnradius 1e+02))
  (Utilities|FlowControl|Sequence
    (:then_0
      (for _array_element (Variables|Default|GetPainting)
        (bind _asbp_painting (Utilities|Casting|CastToBP_Painting _array_element))
        (Default|SpawnfromPainting _asbp_painting)))
    (:then_1
      (for _array_element_2 (Variables|Default|GetInnocentSpawnPoints)
        (Rendering|Debug|DrawDebugBox (Transformation|GetActorLocation _array_element_2) _returnvalue "(R=0.000000,G=0.000000,B=1.000000,A=1.000000)" "0, 0, 0" 1e+02 5.0)
        (for _index (range 0 5)
          (bind _returnvalue_2 (Game|SpawnActorfromClass "/Game/NPC/BP_NPC.BP_NPC_C" (Math|Transform|MakeTransform (Math|Random|RandomPointinBoundingBox (Transformation|GetActorLocation _array_element_2) _returnvalue) (Math|Rotator|MakeRotator 0.0 0.0 (Math|Random|RandomFloatinRange 0.0 1.8e+02)) "1,1,1") "AdjustIfPossibleButDontSpawnIfColliding" 0 0))
          (Utilities|IsValid _returnvalue_2
            (:Is%20Valid
              (Variables|/Game/NPC/BP_NPC.BP_NPC_C|SetEnemy _returnvalue_2 false)
              (Class|SkinnedMeshComponent|SetSkeletalMesh (Variables|/Script/Engine.Character|GetMesh _returnvalue_2) (Utilities|Array|Get(acopy) (Variables|Default|GetAllSkeletalMeshes) (Math|Random|RandomIntegerinRange 0 5)) true))))))))

(event Collision|EventActorBeginOverlap
  (params (OtherActor :type Actor%20Object%20Reference)))

(event EventTick
  (params (DeltaSeconds :type Float%20%28single-precision%29)))

(fn ConstructionScript)