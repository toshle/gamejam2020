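; BP_Splaterrer is an NPC component that produces splatter particles and decals when its OnHit event fires.
; OnHit attaches an emitter to the owner's capsule at the hit point, oriented along the hit direction, and deactivates it on a short timer.
; Each particle collision spawns a temporary decal aligned to the surface normal, with random size and a random Frame parameter on a dynamic material instance for variety.
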(event Custom|OnHit
  (params (Direction :type Vector) (Location :type Vector))
  (bind _returnvalue (Components|GetOwner))
  (bind _returnvalue_2 (Actor|GetComponentbyClass _returnvalue "/Script/Engine.CapsuleComponent"))
  (bind _returnvalue_3 (Effects|SpawnEmitterAttached (Variables|Default|GetSplatterEmitters) _returnvalue_2 "None" (- Location (Transformation|GetWorldLocation _returnvalue_2)) (Math|Conversions|RotationFromXVector Direction)))
  (EventDispatchers|BindEventtoOnParticleCollide _returnvalue_3 (delegate Custom|CustomEvent_1))
  (Utilities|Time|SetTimerbyFunctionName _returnvalue_3 "Deactivate" 2.0))

(event Custom|CustomEvent_1
  (params (EventName :type Name) (EmitterTime :type Float%20%28single-precision%29) (ParticleTime :type Integer) (Location :type Vector) (Velocity :type Vector) (Direction :type Vector) (Normal :type Vector) (BoneName :type Name) (PhysMat :type Physical%20Material%20Object%20Reference))
  ;[1 1 1] Use for later for blood trail
  (bind _returnvalue (Rendering|Material|CreateDynamicMaterialInstance "/Game/NPC/Art/Materials/M_Splatter_Decal.M_Splatter_Decal" :!class /Script/Engine.KismetMaterialLibrary))
  (Rendering|Material|SetScalarParameterValue _returnvalue "Frame" (Math|Conversions|ToFloat(Integer) (Math|Random|RandomInteger 8)) :!class /Script/Engine.MaterialInstanceDynamic)
  (Rendering|Decal|SpawnDecalatLocation _returnvalue (Math|Conversions|ToVector(Float) (Math|Random|RandomFloatinRange 1e+01 2e+01)) Location (Math|Conversions|RotationFromXVector (* Normal -1)) 2e+01))

(event EventBeginPlay)

(event EventTick
  (params (DeltaSeconds :type Float%20%28single-precision%29)))