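; BP_Painting is a painting actor whose depicted enemy leaves it to exist in the level and can later return.
; The construction script applies the empty background and enemy materials to two separate components.
; BeginPlay temporarily handles spawning: it spawns the Enemy class nearby, hides EnemyPainting and registers itself with the enemy's BP_Return_To_Painting_Component.
; ReturnToPainting makes the enemy image visible again.
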(event EventBeginPlay
  (bind _defaultsceneroot (Variables|Default|GetDefaultSceneRoot))
  (bind _returnvalue (Game|SpawnActorfromClass (Variables|Default|GetEnemy) (Math|Conversions|ToTransform(Vector) (+ (Transformation|GetWorldLocation _defaultsceneroot) (+ (Math|Vector|GetForwardVector (Transformation|GetWorldRotation _defaultsceneroot)) "50.000000,50.000000,0.000000"))) "Undefined" 0 0))
  (Development|SetHiddeninGame (Variables|Default|GetEnemyPainting) true false)
  (Variables|/Game/Painting/Blueprints/BP_Return_To_Painting_Component.BP_Return_To_Painting_Component_C|SetPainting (Actor|GetComponentbyClass _returnvalue "/Game/Painting/Blueprints/BP_Return_To_Painting_Component.BP_Return_To_Painting_Component_C") self))

(fn ConstructionScript
  (Rendering|Material|SetMaterial (Variables|Default|GetPaintingBackground) 0 (Variables|Default|GetEmptyPaintingMaterial))
  (Rendering|Material|SetMaterial (Variables|Default|GetEnemyPainting) 0 (Variables|Default|GetEnemyMaterial)))

(fn ReturntoPainting
  (Development|SetHiddeninGame (Variables|Default|GetEnemyPainting) false false))